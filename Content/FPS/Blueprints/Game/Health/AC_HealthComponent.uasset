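; Health component for the FPS game that stores an actor's health between minimum and maximum limits.
; Damage and Heal reject non-positive amounts and write through SetHealth, which clamps; Kill and HealFull pass them huge values.
; Getters expose raw health, normalized health and death state, while Damage also prints health for debugging.
; Init sets health before updating the limits, so that value clamps against the previous bounds.
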(event EventBeginPlay)

(fn Reset
  (Variables|Default|SetHealth (Variables|Default|GetMaxHealth)))

(fn GetHealth
  (return (Variables|Default|GetHealth)))

(fn SetHealth
  (params (New%20Health :type Float%20%28double-precision%29))
  (bind _output_get (Variables|Default|SetHealth (CallFunction|ClampHealth New%20Health)))
  (return _output_get))

(fn PrintHealth
  (Development|PrintString (Utilities|String|ToString(Float) (CallFunction|GetHealth)) true true "(R=1.000000,G=0.019564,B=0.000000,A=1.000000)" 1e+01))

(fn ClampHealth
  (params (Value :type Float%20%28double-precision%29))
  (return (Math|Float|Clamp(Float) Value (Variables|Default|GetMinHealth) (Variables|Default|GetMaxHealth))))

(fn Damage
  (params (DamageAmt :type Float%20%28double-precision%29))
  (if (> DamageAmt 0.0)
    (CallFunction|SetHealth (- (CallFunction|GetHealth) DamageAmt))
    (CallFunction|PrintHealth)
    (else
      (Development|PrintString "Damage value must be positive! Idiot" true true "(R=1.000000,G=0.000000,B=0.019999,A=1.000000)" 1e+01))))

(fn Heal
  (params (HealAmt :type Float%20%28double-precision%29))
  (if (> HealAmt 0.0)
    (CallFunction|SetHealth (+ (CallFunction|GetHealth) HealAmt))
    (else
      (Development|PrintString "Heal value must be positive! Idiot" true true "(R=0.065526,G=1.000000,B=0.003115,A=1.000000)" 1e+01))))

(fn HealFull
  (CallFunction|Heal 1e+25))

(fn Kill
  (CallFunction|Damage 1e+19))

(fn GetNormalziedHealth
  (return (Math|Float|Clamp(Float) (/ (CallFunction|GetHealth) (Variables|Default|GetMaxHealth)))))

(fn IsDead
  (return (<= (CallFunction|GetHealth) (Variables|Default|GetMinHealth))))

(fn Init
  (params (Health :type Float%20%28double-precision%29) (MinHealth :type Float%20%28double-precision%29) (MaxHealth :type Float%20%28double-precision%29))
  (CallFunction|SetHealth Health)
  (Variables|Default|SetMinHealth MinHealth)
  (Variables|Default|SetMaxHealth MaxHealth))