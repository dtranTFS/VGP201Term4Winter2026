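; BP_Player is the first-person player pawn, handling movement, look, jump and gun firing.
; On BeginPlay it spawns the starting gun, snaps it to GunSpawnPoint and caches it as a BPI_Gun interface.
; While Fire is held, PlayerShooting waits the gun's fire rate in a Delay, pacing shots and delaying the first.
; It then sends the gun a camera-forward trace start and end, scaled by the gun's distance.
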(event EventBeginPlay
  (Development|PrintString "Spawning Player" true true "(R=0.000000,G=1.000000,B=0.000000,A=1.000000)" 5.0)
  (CallFunction|SpawnGun (Variables|Default|GetStartingGun)))

(event Input|ActionEvents|InputActionJump
  (params (Key :type Key%20Structure :default "None"))
  ;[0.15 0.15 0.15 0.5] Jump Logic
  (:Pressed
    (Character|Jump)))

(event Input|AxisEvents|InputAxisMoveForward
  (params (AxisValue :type Float%20%28single-precision%29))
  ;[0.15 0.15 0.15 0.5] Move Logic
  (Pawn|Input|AddMovementInput (Transformation|GetActorForwardVector) AxisValue false))

(event Input|AxisEvents|InputAxisHorizontal
  (params (AxisValue :type Float%20%28single-precision%29))
  ;[0.15 0.15 0.15 0.5] Looking Logic
  (Pawn|Input|AddControllerYawInput AxisValue))

(event Input|AxisEvents|InputAxisVertical
  (params (AxisValue :type Float%20%28single-precision%29))
  ;[0.15 0.15 0.15 0.5] Looking Logic
  (Pawn|Input|AddControllerPitchInput AxisValue))

(event Input|AxisEvents|InputAxisFire
  (params (AxisValue :type Float%20%28single-precision%29))
  ;[0.15 0.15 0.15 0.5] Shooting Logic
  (if (> AxisValue 0.0)
    (Utilities|PlayerShooting)))

(event Input|AxisEvents|InputAxisMoveRight
  (params (AxisValue :type Float%20%28single-precision%29))
  ;[0.15 0.15 0.15 0.5] Move Logic
  (Pawn|Input|AddMovementInput (Transformation|GetActorRightVector) AxisValue false))

(fn ConstructionScript)

(fn SpawnGun
  (params (GunToSpawn :type Actor%20Class%20Reference))
  (bind _returnvalue (Game|SpawnActorfromClass GunToSpawn (Math|Transform|MakeTransform "0, 0, 0") "Undefined" "MultiplyWithRoot" 0 0))
  (bind _output_get (Variables|Default|SetGunRef _returnvalue))
  (Transformation|AttachComponentToComponent _output_get (Variables|Default|GetGunSpawnPoint) "None" "SnapToTarget" "SnapToTarget" "SnapToTarget" true)
  (bind _asbpi_gun (Utilities|Casting|CastToBPI_Gun _output_get)
    (:then
      (Variables|Default|SetGunInterfaceRef _asbpi_gun))
    (:CastFailed
      _))
  (return _output_get))

(fn CalculateShoot
  (bind _camera (Variables|Default|GetCamera))
  (bind _returnvalue (Transformation|GetWorldLocation _camera))
  (bind _distance (Default|GetDistance (Variables|Default|GetGunInterfaceRef)))
  (return _returnvalue (+ _returnvalue (* (Math|Vector|GetForwardVector _camera) _distance))))