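; BP_ScoreManager tracks the player's score and shows it in the game menu.
; AddToScore adds only non-negative amounts to Score, then calls UpdateScore, which also runs on BeginPlay.
; UpdateScore casts the game mode to BP_GameMapGameMode and passes the score to its GameMenuRef through SetScore.
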(event EventBeginPlay
  (CallFunction|UpdateScore))

(fn ConstructionScript)

(fn AddtoScore
  (params (Amount :type Integer))
  (Variables|Default|SetScore (+ (Variables|Default|GetScore) (Math|Integer|Clamp(Integer) Amount 0 2147483647)))
  (CallFunction|UpdateScore))

(fn UpdateScore
  (bind _asbp_game_map_game_mode (Utilities|Casting|CastToBP_GameMapGameMode (Game|GetGameMode)))
  (Default|SetScore (Variables|/Game/FPS/Blueprints/Game/Managers/BP_GameMapGameMode.BP_GameMapGameMode_C|GetGameMenuRef _asbp_game_map_game_mode) (Variables|Default|GetScore)))