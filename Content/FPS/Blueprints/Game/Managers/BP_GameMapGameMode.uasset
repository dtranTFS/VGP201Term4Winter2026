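; Game mode for the FPS game map that runs a countdown and signals game over when it expires.
; On BeginPlay it creates the game menu widget, sets game-only input and spawns the score manager.
; Tick runs DecreaseTimer, whose one-second Delay throttles the countdown and refreshes the menu's timer.
; At zero or below it calls the TimerRanOut and GameOver dispatchers, with no guard against repeats.
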(event EventTick
  (params (DeltaSeconds :type Float%20%28single-precision%29))
  (Utilities|DecreaseTimer)
  (if (<= (Variables|Config|GetGameTimer) 0)
    (Default|CallTimerRanOut)
    (Default|CallGameOver)))

(event EventBeginPlay
  (Development|PrintString "Hello World" true true "(R=0.000000,G=0.660000,B=1.000000,A=1.000000)" 5.0)
  (Development|PrintString "Spawning BP_GameMapGameMode" true true "(R=0.000000,G=0.660000,B=1.000000,A=1.000000)" 5.0)
  (CallFunction|SpawnGameMenu)
  (CallFunction|SetInputtoGame)
  (CallFunction|UpdateTimer)
  (bind _returnvalue (Game|SpawnActorfromClass "/Game/FPS/Blueprints/Game/Managers/BP_ScoreManager.BP_ScoreManager_C" (Math|Transform|MakeTransform "0, 0, 0" "0, 0, 0" "1.000000,1.000000,1.000000") "Undefined" "MultiplyWithRoot" 0 0))
  (Variables|Default|SetScoreManagerRef _returnvalue))

(fn ConstructionScript)

(fn SpawnGameMenu
  (bind _returnvalue (UserInterface|CreateWidget "/Game/FPS/Blueprints/Game/GUI/WBP_GameMenu.WBP_GameMenu_C"))
  (bind _output_get (Variables|Default|SetGameMenuRef _returnvalue))
  (UserInterface|Viewport|AddtoViewport _output_get 0))

(fn SetInputtoGame
  (bind _returnvalue (Game|GetPlayerController 0))
  (Input|SetInputModeGameOnly _returnvalue false)
  (Variables|/Script/Engine.PlayerController|SetbShowMouseCursor _returnvalue false))

(fn UpdateTimer
  (Default|SetTimer (Variables|Default|GetGameMenuRef) (Variables|Config|GetGameTimer)))